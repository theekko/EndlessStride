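; BP_FallArea is a map trigger volume that respawns the first-person player who falls into it.
; When its box overlaps a BP_FirstPersonCharacter, it flags the player as died and teleports them to their stored respawn location with zeroed rotation.
; It also resets the projectile count and destroys the first BP_AbilityBase actor found in the world, if any.
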(event OnComponentBeginOverlap(Box)
  (params (OverlappedComponent :type Primitive%20Component%20Object%20Reference) (OtherActor :type Actor%20Object%20Reference) (OtherComp :type Primitive%20Component%20Object%20Reference) (OtherBodyIndex :type Integer) (bFromSweep :type Boolean) (SweepResult :type Hit%20Result%20Structure%20%28by%20ref%29))
  ;[0.05098 0.05098 0.05098] Respawn Player at current respawn point
  (bind _asbp_first_person_character (Utilities|Casting|CastToBP_FirstPersonCharacter OtherActor))
  (Variables|Default|SetAs%20BP%20First%20Person%20Character _asbp_first_person_character)
  (Variables|/Game/Dynamic/GameRules/Blueprints/BP_FirstPersonCharacter.BP_FirstPersonCharacter_C|SetPlayerDied (Variables|Default|GetAs%20BP%20First%20Person%20Character) true)
  (Transformation|Teleport (Variables|Default|GetAs%20BP%20First%20Person%20Character) (Variables|/Game/Dynamic/GameRules/Blueprints/BP_FirstPersonCharacter.BP_FirstPersonCharacter_C|GetRespawnLocation (Variables|Default|GetAs%20BP%20First%20Person%20Character)) "0, 0, 0")
  (Variables|/Game/Dynamic/GameRules/Blueprints/BP_FirstPersonCharacter.BP_FirstPersonCharacter_C|SetProjectileCount (Variables|Default|GetAs%20BP%20First%20Person%20Character) 3.0)
  (bind _outactors (Actor|GetAllActorsOfClass "/Game/Dynamic/Objects/BP_AbilityBase.BP_AbilityBase_C"))
  (if (> (Utilities|Array|Length _outactors) 0)
    (Actor|DestroyActor (Utilities|Array|Get(acopy) _outactors))))

(fn ConstructionScript)
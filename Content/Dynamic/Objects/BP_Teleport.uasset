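; BP_Teleport is a teleport marker actor that moves the player to its own position when its UseAbility event fires.
; The event finds the first BP_FirstPersonCharacter in the level and teleports it to the root component's world location with zero rotation.
; It then sets the character's TeleportJump and CanDash flags and destroys itself, so each instance works once.
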(event EventUseAbility
  ;[0.05098 0.05098 0.05098] Teleport
  (bind _outactors (Actor|GetAllActorsOfClass "/Game/Dynamic/GameRules/Blueprints/BP_FirstPersonCharacter.BP_FirstPersonCharacter_C"))
  (bind _output_get (Variables|Default|SetPlayer (Utilities|Array|Get(acopy) _outactors)))
  (Transformation|Teleport _output_get (Transformation|GetWorldLocation (Variables|Default|GetDefaultSceneRoot self)) "0, 0, 0")
  (Variables|/Game/Dynamic/GameRules/Blueprints/BP_FirstPersonCharacter.BP_FirstPersonCharacter_C|SetTeleportJump _output_get true)
  (Variables|/Game/Dynamic/GameRules/Blueprints/BP_FirstPersonCharacter.BP_FirstPersonCharacter_C|SetCanDash _output_get true)
  (Actor|DestroyActor))

(fn ConstructionScript
  (|CallParentFunction))
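; Fire wall hazard that streams fire projectiles and detects the first-person character crossing it.
; A looping timer spawns BP_EnemyProjectileFireNoCollision from three spouts at a set fire rate.
; Separately, every Tick runs line traces from five spouts along RaycastDistance, ignoring ground-collision actors cached at BeginPlay, and calls HitFireShield on the character when hit.
; Hit detection here thus comes from the traces, independent of the spawned projectiles.
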(event Custom|ShootFire
  (Utilities|FlowControl|Sequence
    (:then_0
      (Game|SpawnActorfromClass "/Game/Dynamic/Projectiles/BP_EnemyProjectileFireNoCollision.BP_EnemyProjectileFireNoCollision_C" (Math|Transform|MakeTransform (Transformation|GetWorldLocation (Variables|Default|GetFireSpout)) "90.000000,0.000000,0.000000" "1.000000,1.000000,1.000000") "Undefined" "MultiplyWithRoot" 0 (Variables|Default|GetProjectileSpeed) 0.0 0 false (Variables|Default|GetDestroyTimer) false (Variables|Default|GetVelocityDirection) 0))
    (:then_1
      (Game|SpawnActorfromClass "/Game/Dynamic/Projectiles/BP_EnemyProjectileFireNoCollision.BP_EnemyProjectileFireNoCollision_C" (Math|Transform|MakeTransform (Transformation|GetWorldLocation (Variables|Default|GetFireSpout1)) "90.000000,0.000000,0.000000" "1.000000,1.000000,1.000000") "Undefined" "MultiplyWithRoot" 0 (Variables|Default|GetProjectileSpeed) 0.0 0 false (Variables|Default|GetDestroyTimer) false (Variables|Default|GetVelocityDirection) 0))
    (:then_2
      (Game|SpawnActorfromClass "/Game/Dynamic/Projectiles/BP_EnemyProjectileFireNoCollision.BP_EnemyProjectileFireNoCollision_C" (Math|Transform|MakeTransform (Transformation|GetWorldLocation (Variables|Default|GetFireSpout2)) "90.000000,0.000000,0.000000" "1.000000,1.000000,1.000000") "Undefined" "MultiplyWithRoot" 0 (Variables|Default|GetProjectileSpeed) 0.0 0 false (Variables|Default|GetDestroyTimer) false (Variables|Default|GetVelocityDirection) 0))))

(event EventBeginPlay
  (bind _outactors (Actor|GetAllActorsOfClass "/Game/Static/Maps/MapObjects/BP_GroundCollision.BP_GroundCollision_C"))
  (Variables|Default|SetGroundCollisions _outactors)
  (Utilities|Time|SetTimerbyEvent (delegate Custom|ShootFire) (Variables|Default|GetFireRate%28sec%29) true))

(event EventTick
  (params (DeltaSeconds :type Float%20%28single-precision%29))
  (bind _firespout (Variables|Default|GetFireSpout))
  (bind _firespout1 (Variables|Default|GetFireSpout1))
  (bind _firespout2 (Variables|Default|GetFireSpout2))
  (bind _firespout3 (Variables|Default|GetFireSpout3))
  (bind _firespout4 (Variables|Default|GetFireSpout4))
  (bind _returnvalue (Transformation|GetWorldLocation _firespout4))
  (bind _returnvalue_2 (Transformation|GetWorldLocation _firespout))
  (bind _returnvalue_3 (Transformation|GetWorldLocation _firespout1))
  (bind _returnvalue_4 (Transformation|GetWorldLocation _firespout2))
  (bind _returnvalue_5 (Transformation|GetWorldLocation _firespout3))
  (Utilities|FlowControl|Sequence
    (:then_0
      (bind _outhit (Collision|LineTraceByChannel _returnvalue_2 (+ _returnvalue_2 (Variables|Default|GetRaycastDistance)) "TraceTypeQuery1" false (Variables|Default|GetGroundCollisions) "None"))
      (bind _asbp_first_person_character (Utilities|Casting|CastToBP_FirstPersonCharacter (.HitActor (Collision|BreakHitResult _outhit))))
      (Default|HitFireShield _asbp_first_person_character))
    (:then_1
      (bind _outhit_2 (Collision|LineTraceByChannel _returnvalue_3 (+ _returnvalue_3 (Variables|Default|GetRaycastDistance)) "TraceTypeQuery1" false (Variables|Default|GetGroundCollisions) "None"))
      (bind _asbp_first_person_character_2 (Utilities|Casting|CastToBP_FirstPersonCharacter (.HitActor (Collision|BreakHitResult _outhit_2))))
      (Default|HitFireShield _asbp_first_person_character_2))
    (:then_2
      (bind _outhit_3 (Collision|LineTraceByChannel _returnvalue_4 (+ _returnvalue_4 (Variables|Default|GetRaycastDistance)) "TraceTypeQuery1" false (Variables|Default|GetGroundCollisions) "None"))
      (bind _asbp_first_person_character_3 (Utilities|Casting|CastToBP_FirstPersonCharacter (.HitActor (Collision|BreakHitResult _outhit_3))))
      (Default|HitFireShield _asbp_first_person_character_3))
    (:then_3
      (bind _outhit_4 (Collision|LineTraceByChannel _returnvalue_5 (+ _returnvalue_5 (Variables|Default|GetRaycastDistance)) "TraceTypeQuery1" false (Variables|Default|GetGroundCollisions) "None"))
      (bind _asbp_first_person_character_4 (Utilities|Casting|CastToBP_FirstPersonCharacter (.HitActor (Collision|BreakHitResult _outhit_4))))
      (Default|HitFireShield _asbp_first_person_character_4))
    (:then_4
      (bind _outhit_5 (Collision|LineTraceByChannel _returnvalue (+ _returnvalue (Variables|Default|GetRaycastDistance)) "TraceTypeQuery1" false (Variables|Default|GetGroundCollisions) "None"))
      (bind _asbp_first_person_character_5 (Utilities|Casting|CastToBP_FirstPersonCharacter (.HitActor (Collision|BreakHitResult _outhit_5))))
      (Default|HitFireShield _asbp_first_person_character_5))))

(fn ConstructionScript)
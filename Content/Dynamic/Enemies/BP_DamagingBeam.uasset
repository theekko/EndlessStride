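; BP_DamagingBeam is an enemy-related emitter that fires a set of seven damaging beams when its activation event is called.
; The event spawns one actor of the configurable BeamType class at the world location and rotation of each of seven Arrow components.
; A Long flag selects between a long and short BeamEnd vector along local X, which is passed to every spawned beam.
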(event Custom|ActivateDamgagingBeam
  (bind _arrow (Variables|Default|GetArrow))
  (bind _arrow1 (Variables|Default|GetArrow1))
  (bind _arrow2 (Variables|Default|GetArrow2))
  (bind _arrow3 (Variables|Default|GetArrow3))
  (bind _arrow4 (Variables|Default|GetArrow4))
  (bind _arrow5 (Variables|Default|GetArrow5))
  (bind _arrow6 (Variables|Default|GetArrow6))
  (if (Variables|Default|GetLong)
    (Variables|Default|SetBeamEnd "16000.000000,0.000000,0.000000")
    (else
      (Variables|Default|SetBeamEnd "6000.000000,0.000000,0.000000")))
  (Game|SpawnActorfromClass (Variables|Default|GetBeamType) (Math|Transform|MakeTransform (Transformation|GetWorldLocation _arrow) (Transformation|GetWorldRotation _arrow) "1.000000,1.000000,1.000000") "Undefined" "MultiplyWithRoot" 0 (Variables|Default|GetBeamEnd) 0)
  (Game|SpawnActorfromClass (Variables|Default|GetBeamType) (Math|Transform|MakeTransform (Transformation|GetWorldLocation _arrow1) (Transformation|GetWorldRotation _arrow1) "1.000000,1.000000,1.000000") "Undefined" "MultiplyWithRoot" 0 (Variables|Default|GetBeamEnd) 0)
  (Game|SpawnActorfromClass (Variables|Default|GetBeamType) (Math|Transform|MakeTransform (Transformation|GetWorldLocation _arrow2) (Transformation|GetWorldRotation _arrow2) "1.000000,1.000000,1.000000") "Undefined" "MultiplyWithRoot" 0 (Variables|Default|GetBeamEnd) 0)
  (Game|SpawnActorfromClass (Variables|Default|GetBeamType) (Math|Transform|MakeTransform (Transformation|GetWorldLocation _arrow3) (Transformation|GetWorldRotation _arrow3) "1.000000,1.000000,1.000000") "Undefined" "MultiplyWithRoot" 0 (Variables|Default|GetBeamEnd) 0)
  (Game|SpawnActorfromClass (Variables|Default|GetBeamType) (Math|Transform|MakeTransform (Transformation|GetWorldLocation _arrow4) (Transformation|GetWorldRotation _arrow4) "1.000000,1.000000,1.000000") "Undefined" "MultiplyWithRoot" 0 (Variables|Default|GetBeamEnd) 0)
  (Game|SpawnActorfromClass (Variables|Default|GetBeamType) (Math|Transform|MakeTransform (Transformation|GetWorldLocation _arrow5) (Transformation|GetWorldRotation _arrow5) "1.000000,1.000000,1.000000") "Undefined" "MultiplyWithRoot" 0 (Variables|Default|GetBeamEnd) 0)
  (Game|SpawnActorfromClass (Variables|Default|GetBeamType) (Math|Transform|MakeTransform (Transformation|GetWorldLocation _arrow6) (Transformation|GetWorldRotation _arrow6) "1.000000,1.000000,1.000000") "Undefined" "MultiplyWithRoot" 0 (Variables|Default|GetBeamEnd) 0))

(fn ConstructionScript)
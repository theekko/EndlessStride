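; BP_FireCylinder is an enemy attack actor that forms a cylinder of fire projectiles around its location.
; On BeginPlay, nested loops place BP_EnemyProjectileFire actors in rings by trigonometry, each facing the central axis.
; Layer heights start at world Z zero, ignoring the actor's own height.
; Projectiles spawn with zero speed, the first-person character as target and a short destroy timer.
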(event EventBeginPlay
  (bind _defaultsceneroot (Variables|Default|GetDefaultSceneRoot))
  (bind _defaultsceneroot_2 (Variables|Default|GetDefaultSceneRoot))
  (bind _returnvalue (Transformation|GetWorldLocation _defaultsceneroot))
  (bind _returnvalue_2 (Transformation|GetWorldLocation _defaultsceneroot_2))
  (bind _returnvalue_3 (Actor|GetActorOfClass "/Game/Dynamic/GameRules/Blueprints/BP_FirstPersonCharacter.BP_FirstPersonCharacter_C"))
  (Variables|Default|SetPlayer _returnvalue_3)
  (for _index (range 0 (Math|Float|Truncate (Variables|Default|GetNumberOfLayers)))
    (Variables|Default|SetZPosition (* _index (/ (Variables|Default|GetHeight) (- (Variables|Default|GetNumberOfLayers) 1))))
    (for _index_2 (range 0 (Math|Float|Truncate (Variables|Default|GetPointsPerLayer)))
      (bind _output_get (Variables|Default|SetAngle (* 3.6e+02 (/ _index_2 (Variables|Default|GetPointsPerLayer)))))
      (Variables|Default|SetAngle (* _output_get (/ (Math|Trig|GetPI) 1.8e+02)))
      (Game|SpawnActorfromClass "/Game/Dynamic/Projectiles/BP_EnemyProjectileFire.BP_EnemyProjectileFire_C" (Math|Transform|MakeTransform (Math|Vector|MakeVector (+ (.x _returnvalue_2) (* (Variables|Default|GetRadius) (Math|Trig|Cos(Radians) (Variables|Default|GetAngle)))) (+ (.y _returnvalue_2) (* (Variables|Default|GetRadius) (Math|Trig|Sin(Radians) (Variables|Default|GetAngle)))) (Variables|Default|GetZPosition)) (Math|Rotator|FindLookatRotation (Math|Vector|MakeVector (+ (.x _returnvalue_2) (* (Variables|Default|GetRadius) (Math|Trig|Cos(Radians) (Variables|Default|GetAngle)))) (+ (.y _returnvalue_2) (* (Variables|Default|GetRadius) (Math|Trig|Sin(Radians) (Variables|Default|GetAngle)))) (Variables|Default|GetZPosition)) (Math|Vector|MakeVector (.x _returnvalue) (.y _returnvalue) (Variables|Default|GetZPosition))) "1.000000,1.000000,1.000000") "Undefined" "MultiplyWithRoot" 0 0.0 0.0 (Variables|Default|GetPlayer) false 3.0 true "0.000000,0.000000,0.000000" 0))))

(fn ConstructionScript)
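; BP_ChargingBeam is an enemy charge-beam effect Blueprint.
; Its ActivateChargeBeam event checks the Long flag and activates one of two separate sets of seven NSBeam components without resetting them.
; The graph only handles activation, with no deactivation, timing or damage logic, and the construction script is empty.
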(event Custom|ActivateChargeBeam
  (if (Variables|Default|Getlong)
    (Components|Activation|Activate (Variables|Default|GetNS_Beam) false)
    (Components|Activation|Activate (Variables|Default|GetNS_Beam_01) false)
    (Components|Activation|Activate (Variables|Default|GetNS_Beam_02) false)
    (Components|Activation|Activate (Variables|Default|GetNS_Beam_03) false)
    (Components|Activation|Activate (Variables|Default|GetNS_Beam_04) false)
    (Components|Activation|Activate (Variables|Default|GetNS_Beam_05) false)
    (Components|Activation|Activate (Variables|Default|GetNS_Beam_06) false)
    (else
      (Components|Activation|Activate (Variables|Default|GetNS_Beam_07) false)
      (Components|Activation|Activate (Variables|Default|GetNS_Beam_08) false)
      (Components|Activation|Activate (Variables|Default|GetNS_Beam_09) false)
      (Components|Activation|Activate (Variables|Default|GetNS_Beam_010) false)
      (Components|Activation|Activate (Variables|Default|GetNS_Beam_011) false)
      (Components|Activation|Activate (Variables|Default|GetNS_Beam_012) false)
      (Components|Activation|Activate (Variables|Default|GetNS_Beam_013) false))))

(fn ConstructionScript)
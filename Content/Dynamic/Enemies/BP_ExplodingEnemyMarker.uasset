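; Exploding enemy marker that surrounds its location with two orbiting rings of BP_ExplodingMarkerSection actors.
; BeginPlay spawns both rings evenly spaced by NumEmitters and maps each section to its angle.
; While EnemyExists, Tick advances those angles and repositions sections with sine/cosine offsets, rotated by separate normal and inverted angles around the root's location vector.
; EnemyHit clears EnemyExists, prints a debug message and destroys every section.
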(event Custom|EnemyHit
  ;[0.05098 0.05098 0.05098] DestroySections
  (Variables|Default|SetEnemyExists false)
  (Development|PrintString "Hit")
  (for _array_element (Variables|Default|GetMarkerSections)
    (Actor|DestroyActor _array_element))
  (for _array_element_2 (Variables|Default|GetMarkerSectionsInverted)
    (Actor|DestroyActor _array_element_2)))

(event EventBeginPlay
  ;[0.05098 0.05098 0.05098] Spawn Sections
  (for _index (range 0 (Math|Float|Truncate (- (Variables|Default|GetNumEmitters) 1.0)))
    (CallFunction|SpawnExplodingMarkerSections _index))
  (for _index_2 (range 0 (Math|Float|Truncate (- (Variables|Default|GetNumEmitters) 1.0)))
    (CallFunction|SpawnExplodingMarkerSectionsInverted _index_2)))

(event EventTick
  (params (DeltaSeconds :type Float%20%28single-precision%29))
  ;[0.05098 0.05098 0.05098] Rotate Sections
  (if (Variables|Default|GetEnemyExists)
    (CallFunction|RotateSections DeltaSeconds)
    (CallFunction|RotateInvertedSections DeltaSeconds)))

(fn ConstructionScript)

(fn SpawnExplodingMarkerSections
  (params (A :type Integer))
  (bind _defaultsceneroot (Variables|Default|GetDefaultSceneRoot))
  (bind _returnvalue (Transformation|GetWorldLocation _defaultsceneroot))
  (Variables|Default|SetCurrentAngle (* 3.6e+02 (/ A (Variables|Default|GetNumEmitters))))
  (bind _returnvalue_2 (Game|SpawnActorfromClass "/Game/Dynamic/Enemies/BP_ExplodingMarkerSection.BP_ExplodingMarkerSection_C" (Math|Transform|MakeTransform (Math|Vector|RotateVectorAroundAxis (+ _returnvalue (Math|Vector|MakeVector (* (Variables|Default|GetRadius) (Math|Trig|Cos(Degrees) (Variables|Default|GetCurrentAngle))) (* (Variables|Default|GetRadius) (Math|Trig|Sin(Degrees) (Variables|Default|GetCurrentAngle))) 0.0)) 25.0 _returnvalue) "0, 0, 0" "1.000000,1.000000,1.000000") "Undefined" "MultiplyWithRoot" 0 0))
  (Utilities|Map|Add (Variables|Default|GetMarkerSectionsToAngle) _returnvalue_2 (Variables|Default|GetCurrentAngle))
  (Utilities|Array|Add (Variables|Default|GetMarkerSections) _returnvalue_2))

(fn SpawnExplodingMarkerSectionsInverted
  (params (A :type Integer))
  (bind _defaultsceneroot (Variables|Default|GetDefaultSceneRoot))
  (bind _relativelocation (Variables|/Script/Engine.SceneComponent|GetRelativeLocation _defaultsceneroot))
  (Variables|Default|SetCurrentAngle (* 3.6e+02 (/ A (Variables|Default|GetNumEmitters))))
  (bind _returnvalue (Game|SpawnActorfromClass "/Game/Dynamic/Enemies/BP_ExplodingMarkerSection.BP_ExplodingMarkerSection_C" (Math|Transform|MakeTransform (Math|Vector|RotateVectorAroundAxis (+ _relativelocation (Math|Vector|MakeVector (* (Variables|Default|GetRadius) (Math|Trig|Cos(Degrees) (Variables|Default|GetCurrentAngle))) (* (Variables|Default|GetRadius) (Math|Trig|Sin(Degrees) (Variables|Default|GetCurrentAngle))) 0.0)) (Variables|Default|GetRotationAngleInverted) _relativelocation) "0, 0, 0" "1.000000,1.000000,1.000000") "Undefined" "MultiplyWithRoot" 0 0))
  (Utilities|Map|Add (Variables|Default|GetMarkerSectionsToAngleInverted) _returnvalue (Variables|Default|GetCurrentAngle))
  (Utilities|Array|Add (Variables|Default|GetMarkerSectionsInverted) _returnvalue))

(fn RotateSections
  (params (A :type Float%20%28double-precision%29))
  (bind _defaultsceneroot (Variables|Default|GetDefaultSceneRoot))
  (bind _returnvalue (Transformation|GetWorldLocation _defaultsceneroot))
  (for _array_element (Variables|Default|GetMarkerSections)
    (Variables|Default|SetCurrentMarkerSection _array_element)
    (Transformation|SetActorLocation _array_element (Math|Vector|RotateVectorAroundAxis (+ _returnvalue (Math|Vector|MakeVector (* (Variables|Default|GetRadius) (Math|Trig|Cos(Degrees) (+ (.Value (Utilities|Map|Find (Variables|Default|GetMarkerSectionsToAngle) (Variables|Default|GetCurrentMarkerSection))) (* A (Variables|Default|GetRotationSpeed))))) (* (Variables|Default|GetRadius) (Math|Trig|Sin(Degrees) (+ (.Value (Utilities|Map|Find (Variables|Default|GetMarkerSectionsToAngle) (Variables|Default|GetCurrentMarkerSection))) (* A (Variables|Default|GetRotationSpeed))))) 0.0)) (Variables|Default|GetRotationAngle) _returnvalue) false false)
    (Utilities|Map|Add (Variables|Default|GetMarkerSectionsToAngle) (Variables|Default|GetCurrentMarkerSection) (+ (.Value (Utilities|Map|Find (Variables|Default|GetMarkerSectionsToAngle) (Variables|Default|GetCurrentMarkerSection))) (* A (Variables|Default|GetRotationSpeed))))))

(fn RotateInvertedSections
  (params (InputPin :type Float%20%28single-precision%29))
  (bind _defaultsceneroot (Variables|Default|GetDefaultSceneRoot))
  (bind _returnvalue (Transformation|GetWorldLocation _defaultsceneroot))
  (for _array_element (Variables|Default|GetMarkerSectionsInverted)
    (Variables|Default|SetCurrentMarkerSection _array_element)
    (Transformation|SetActorLocation _array_element (Math|Vector|RotateVectorAroundAxis (+ _returnvalue (Math|Vector|MakeVector (* (Variables|Default|GetRadius) (Math|Trig|Cos(Degrees) (+ (.Value (Utilities|Map|Find (Variables|Default|GetMarkerSectionsToAngleInverted) (Variables|Default|GetCurrentMarkerSection))) (* InputPin (Variables|Default|GetRotationSpeed))))) (* (Variables|Default|GetRadius) (Math|Trig|Sin(Degrees) (+ (.Value (Utilities|Map|Find (Variables|Default|GetMarkerSectionsToAngleInverted) (Variables|Default|GetCurrentMarkerSection))) (* InputPin (Variables|Default|GetRotationSpeed))))) 0.0)) (Variables|Default|GetRotationAngleInverted) _returnvalue) false false)
    (Utilities|Map|Add (Variables|Default|GetMarkerSectionsToAngleInverted) (Variables|Default|GetCurrentMarkerSection) (+ (.Value (Utilities|Map|Find (Variables|Default|GetMarkerSectionsToAngleInverted) (Variables|Default|GetCurrentMarkerSection))) (* InputPin (Variables|Default|GetRotationSpeed))))))
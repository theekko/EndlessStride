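; Electric floor hazard that an enemy attack can switch on to hurt the first-person player standing inside its cube.
; ActivateAttack shows the cube with a charging material, then after a ChargingTime delay switches to the active material and arms it; DeactivateAttack hides and disarms it.
; Cube overlap events track whether the player is inside, and Tick calls HitElectricField on the player every frame while both conditions hold.
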(event OnComponentBeginOverlap(Cube)
  (params (OverlappedComponent :type Primitive%20Component%20Object%20Reference) (OtherActor :type Actor%20Object%20Reference) (OtherComp :type Primitive%20Component%20Object%20Reference) (OtherBodyIndex :type Integer) (bFromSweep :type Boolean) (SweepResult :type Hit%20Result%20Structure%20%28by%20ref%29))
  (Utilities|Casting|CastToBP_FirstPersonCharacter OtherActor)
  (Variables|Default|SetPlayerOverlapping true))

(event OnComponentEndOverlap(Cube)
  (params (OverlappedComponent :type Primitive%20Component%20Object%20Reference) (OtherActor :type Actor%20Object%20Reference) (OtherComp :type Primitive%20Component%20Object%20Reference) (OtherBodyIndex :type Integer))
  (Utilities|Casting|CastToBP_FirstPersonCharacter OtherActor)
  (Variables|Default|SetPlayerOverlapping false))

(event Custom|ActivateAttack
  (Rendering|Material|SetMaterial (Variables|Default|GetCube) 0 "/Game/Dynamic/Materials/MT_ElectricityCharging.MT_ElectricityCharging")
  (Rendering|SetVisibility (Variables|Default|GetCube) true false)
  (Utilities|FlowControl|Delay (Variables|Default|GetChargingTime))
  (Rendering|Material|SetMaterial (Variables|Default|GetCube) 0 "/Game/Dynamic/Materials/MT_ElectricityActive.MT_ElectricityActive")
  (Variables|Default|SetActivated true))

(event Custom|DeactivateAttack
  (Rendering|SetVisibility (Variables|Default|GetCube) false false)
  (Variables|Default|SetActivated false))

(event EventBeginPlay
  (Rendering|SetVisibility (Variables|Default|GetCube) false false))

(event EventTick
  (params (DeltaSeconds :type Float%20%28single-precision%29))
  (if (and (Variables|Default|GetActivated) (Variables|Default|GetPlayerOverlapping))
    (bind _returnvalue (Actor|GetActorOfClass "/Game/Dynamic/GameRules/Blueprints/BP_FirstPersonCharacter.BP_FirstPersonCharacter_C"))
    (Default|HitElectricField _returnvalue)))

(fn ConstructionScript)
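; BP_FireShield is a temporary flame shield, filed under enemies, that shrinks after a delay and then destroys itself.
; On BeginPlay it caches the first-person player character and the shield's starting world scale, then waits TimeBeforeShrink.
; A Timeline then multiplies that starting scale by its ShieldSize track, and the actor is destroyed when the Timeline finishes.
; The cached player reference is not used in these graphs.
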(event EventBeginPlay
  (bind _returnvalue (Actor|GetActorOfClass "/Game/Dynamic/GameRules/Blueprints/BP_FirstPersonCharacter.BP_FirstPersonCharacter_C"))
  (Variables|Default|SetPlayer _returnvalue)
  (Variables|Default|SetCurrentFlameShieldScale (Transformation|GetWorldScale (Variables|Default|GetFlameShield)))
  (Utilities|FlowControl|Delay (Variables|Default|GetTimeBeforeShrink))
  (bind _shieldsize (Timeline|Timeline PlayFromStart)
    (:Update
      (Transformation|SetWorldScale3D (Variables|Default|GetFlameShield) (* (Variables|Default|GetCurrentFlameShieldScale) _shieldsize)))
    (:Finished
      (Actor|DestroyActor))))

(fn ConstructionScript)
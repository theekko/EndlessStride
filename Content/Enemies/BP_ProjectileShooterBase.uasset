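; Base shooter enemy that fires a configurable, optionally homing projectile at the first-person player on a looping timer.
; A player projectile hitting its box replaces the first existing ability actor, if any, with a new ability point at that location.
; Any box hit, whatever the source, optionally fires a death projectile at the player, reports the death to SectionSeparator and destroys the enemy.
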(event OnComponentHit(Box)
  (params (HitComponent :type Primitive%20Component%20Object%20Reference) (OtherActor :type Actor%20Object%20Reference) (OtherComp :type Primitive%20Component%20Object%20Reference) (NormalImpulse :type Vector :default "0, 0, 0") (Hit :type Hit%20Result%20Structure%20%28by%20ref%29))
  ;[0.05098 0.05098 0.05098] Destroy actor and spawn teleport point and death projectile
  (Utilities|FlowControl|Sequence
    (:then_0
      (Utilities|Casting|CastToBP_PlayerProjectileBase OtherActor)
      (bind _outactors (Actor|GetAllActorsOfClass "/Game/Objects/BP_AbilityBase.BP_AbilityBase_C"))
      (if (> (Utilities|Array|Length _outactors) 0)
        (Actor|DestroyActor (Utilities|Array|Get(acopy) _outactors)))
      (Game|SpawnActorfromClass (Variables|Default|GetAbilityPointSpawn) (Math|Transform|MakeTransform (Transformation|GetWorldLocation (Variables|Default|GetBox)) "0, 0, 0" "1.000000,1.000000,1.000000") "Undefined" "MultiplyWithRoot" 0 (Variables|Default|GetGravityDirection) (Variables|Default|GetForwardDirection) 0))
    (:then_1
      (if (Variables|Default|GetDeathProjectile)
        (Game|SpawnActorfromClass (Variables|Projectile|GetProjectileType) (Math|Transform|MakeTransform (Transformation|GetWorldLocation (Variables|Default|GetArrow))) "Undefined" "MultiplyWithRoot" self (Variables|Default|GetDeathProjectileSpeed) 0.0 (Variables|Default|GetPlayer) false (Variables|Default|GetDeathProjectileDestroyTimer) 0))
      (Default|EnemyDeath (Variables|Default|GetSectionSeparator))
      (Actor|DestroyActor))))

(event Custom|Shoot
  ;[0.05098 0.05098 0.05098] Shoot Projectile at target on timer
  (Game|SpawnActorfromClass (Variables|Projectile|GetProjectileType) (Math|Transform|MakeTransform (Transformation|GetWorldLocation (Variables|Default|GetArrow))) "Undefined" "MultiplyWithRoot" self (Variables|Projectile|GetSpeed) 0.0 (Variables|Default|GetPlayer) (Variables|Projectile|GetIsHoming) (Variables|Default|GetDestroyTimer) 0))

(event EventBeginPlay
  ;[0.05098 0.05098 0.05098] Shoot Projectile at target on timer
  (bind _returnvalue (Actor|GetActorOfClass "/Game/FirstPerson/Blueprints/BP_FirstPersonCharacter.BP_FirstPersonCharacter_C"))
  (Variables|Default|SetPlayer _returnvalue)
  (Utilities|Time|SetTimerbyEvent (delegate Custom|Shoot) (Variables|Projectile|GetFrequency) true))

(fn ConstructionScript)
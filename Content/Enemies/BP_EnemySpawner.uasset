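; Enemy spawner that places a projectile shooter enemy at its location when its linked checkpoint fires the spawn event, intended for threshold crossings and deaths.
; On BeginPlay it casts SpawnEnemyTrigger to BP_Checkpoint and binds to that event.
; Each trigger destroys any previously spawned shooter still valid, then spawns a fresh one configured from the spawner's own projectile, timer, death-projectile and orientation variables.
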(event Custom|SpawnEnemiesEvent_Event
  ;[0.05098 0.05098 0.05098] Spawn enemies on player passing through threshold and on death
  (if (Variables|Default|GetSpawnedEnemy)
    (Utilities|IsValid (stale _returnvalue)
      (:Is%20Valid
        (Actor|DestroyActor (stale _returnvalue)))
      (:Is%20Not%20Valid
        _)))
  (bind _returnvalue (Game|SpawnActorfromClass "/Game/Enemies/BP_ProjectileShooterBase.BP_ProjectileShooterBase_C" (Math|Transform|MakeTransform (Transformation|GetWorldLocation (Variables|Default|GetDefaultSceneRoot self)) (Variables|Default|GetSpawnRotation) "1.000000,1.000000,1.000000") "Undefined" "MultiplyWithRoot" 0 (Variables|Default|GetFrequency) (Variables|Default|GetProjectile%20Type) (Variables|Default|GetHoming) (Variables|Default|GetProjectileSpeed) (Variables|Default|GetAbility%20Point%20Spawn) (Variables|Default|GetSectionSeparator) (Variables|Default|GetDestroy%20Timer) (Variables|Default|GetDeathProjectileTimer) (Variables|Default|GetDeathProjectileSpeed) (Variables|Default|GetDeathProjectile) (Variables|Default|GetGravityDirection) (Variables|Default|GetForwardDirection) 0))
  (Variables|Default|SetSpawnedEnemy true))

(event EventBeginPlay
  ;[0.05098 0.05098 0.05098] Spawn enemies on player passing through threshold and on death
  (bind _asbp_checkpoint (Utilities|Casting|CastToBP_Checkpoint (Variables|Default|GetSpawnEnemyTrigger)))
  (EventDispatchers|AssignSpawnEnemiesEvent _asbp_checkpoint (delegate Custom|SpawnEnemiesEvent_Event)))

(fn ConstructionScript)
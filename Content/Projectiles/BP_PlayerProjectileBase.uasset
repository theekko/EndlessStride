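; Base player projectile that destroys itself on any hit and signals when it strikes an enemy.
; The construction script feeds speed and gravity into ProjectileMovement and enables homing on the target's root component when flagged and valid.
; On BeginPlay its Box ignores the owner while moving.
; Hits identify enemies by comparing the collision object type's name to "Enemy", call OnEnemyProjectileImpact for those, and print debug strings.
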(event OnComponentHit(Box)
  (params (HitComponent :type Primitive%20Component%20Object%20Reference) (OtherActor :type Actor%20Object%20Reference) (OtherComp :type Primitive%20Component%20Object%20Reference) (NormalImpulse :type Vector :default "0, 0, 0") (Hit :type Hit%20Result%20Structure%20%28by%20ref%29))
  ;[0.05098 0.05098 0.05098] Destroy on impact, detect enemy impact
  (if (Utilities|Enum|Equal(Enum) (Utilities|String|EnumtoString (Collision|GetCollisionObjectType OtherComp)) "Enemy")
    (Default|CallOnEnemyProjectileImpact)
    (Actor|DestroyActor)
    (Development|PrintString "Enemy")
    (else
      (Actor|DestroyActor)
      (Development|PrintString "NotEnemy"))))

(event EventBeginPlay
  ;[0.05098 0.05098 0.05098] Projectile Ignore Player
  (Collision|IgnoreActorwhenMoving (Variables|Default|GetBox) (Components|GetOwner) true))

(fn ConstructionScript
  (bind _projectilemovement (Variables|Default|GetProjectileMovement))
  (Utilities|FlowControl|Sequence
    (:then_0
      (Variables|/Script/Engine.ProjectileMovementComponent|SetInitialSpeed _projectilemovement (Variables|ProjectileSettings|GetSpeed))
      (Variables|/Script/Engine.ProjectileMovementComponent|SetMaxSpeed _projectilemovement (Variables|ProjectileSettings|GetSpeed))
      (Variables|/Script/Engine.ProjectileMovementComponent|SetProjectileGravityScale _projectilemovement (Variables|ProjectileSettings|GetGravity)))
    (:then_1
      (Variables|Target|GetTarget
        (:then
          (if (Variables|ProjectileSettings|GetIsHoming)
            (Variables|/Script/Engine.ProjectileMovementComponent|SetbIsHomingProjectile _projectilemovement true)
            (Variables|/Script/Engine.ProjectileMovementComponent|SetHomingTargetComponent _projectilemovement (Variables|/Script/Engine.Actor|GetRootComponent (Variables|Target|GetTarget)))))
        (:else)))))
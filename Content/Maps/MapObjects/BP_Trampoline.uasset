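; BP_Trampoline is a map object that launches the first-person player on overlap with its spring surface and re-enables their dash.
; LaunchDirection is tested against up, down and both Y directions (X is not handled), with LaunchVelocity applied opposite to that vector.
; The launched axis overrides current velocity (Z alone or XY together), while the remaining components take the player's unit forward vector values.
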(event OnComponentBeginOverlap(SpringSurface)
  (params (OverlappedComponent :type Primitive%20Component%20Object%20Reference) (OtherActor :type Actor%20Object%20Reference) (OtherComp :type Primitive%20Component%20Object%20Reference) (OtherBodyIndex :type Integer) (bFromSweep :type Boolean) (SweepResult :type Hit%20Result%20Structure%20%28by%20ref%29))
  (bind _asbp_first_person_character (Utilities|Casting|CastToBP_FirstPersonCharacter OtherActor))
  (bind _output_get (Variables|Default|SetPlayer _asbp_first_person_character))
  (Variables|/Game/FirstPerson/Blueprints/BP_FirstPersonCharacter.BP_FirstPersonCharacter_C|SetCanDash _output_get true)
  (Utilities|FlowControl|Sequence
    (:then_0
      (if (Utilities|Operators|EqualEqual (Variables|Default|GetLaunchDirection) "0.000000,0.000000,1.000000" 0.0)
        (Character|LaunchCharacter (Variables|Default|GetPlayer) (Math|Vector|MakeVector (.x (Transformation|GetActorForwardVector (Variables|Default|GetPlayer))) (.y (Transformation|GetActorForwardVector (Variables|Default|GetPlayer))) (* (Variables|Default|GetLaunchVelocity) -1.0)) false true)))
    (:then_1
      (if (Utilities|Operators|EqualEqual (Variables|Default|GetLaunchDirection) "0.000000,0.000000,-1.000000" 0.0)
        (Character|LaunchCharacter (Variables|Default|GetPlayer) (Math|Vector|MakeVector (.x (Transformation|GetActorForwardVector (Variables|Default|GetPlayer))) (.y (Transformation|GetActorForwardVector (Variables|Default|GetPlayer))) (Variables|Default|GetLaunchVelocity)) false true)))
    (:then_2
      (if (Utilities|Operators|EqualEqual (Variables|Default|GetLaunchDirection) "0.000000,1.000000,0.000000" 0.0)
        (Character|LaunchCharacter (Variables|Default|GetPlayer) (Math|Vector|MakeVector (.x (Transformation|GetActorForwardVector (Variables|Default|GetPlayer))) (* (Variables|Default|GetLaunchVelocity) -1.0) (.z (Transformation|GetActorForwardVector (Variables|Default|GetPlayer)))) true false)))
    (:then_3
      (if (Utilities|Operators|EqualEqual (Variables|Default|GetLaunchDirection) "0.000000,-1.000000,0.000000" 0.0)
        (Character|LaunchCharacter (Variables|Default|GetPlayer) (Math|Vector|MakeVector (.x (Transformation|GetActorForwardVector (Variables|Default|GetPlayer))) (Variables|Default|GetLaunchVelocity) (.z (Transformation|GetActorForwardVector (Variables|Default|GetPlayer)))) true false)))))

(fn ConstructionScript)
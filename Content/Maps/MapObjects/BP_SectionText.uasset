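; BP_SectionText is a map text actor that shows how many spawn points its Section has.
; On BeginPlay it writes the Section's NumSpawnPoints to a TextRender and binds to two Section dispatchers.
; The spawn-count update event rewrites the text, and the destroy-wall event destroys the actor.
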(event Custom|NumSpawnUpdate_Event
  ;[0.05098 0.05098 0.05098] Update Text
  (Rendering|Components|TextRender|SetText (Variables|Default|GetTextRender) (Utilities|Text|ToText(Integer) (Variables|/Game/Maps/MapObjects/BP_SectionSeparator.BP_SectionSeparator_C|GetNumSpawnPoints (Variables|Default|GetSection))))
  (EventDispatchers|AssignNumSpawnUpdate (Variables|Default|GetSection) (delegate Custom|NumSpawnUpdate_Event))
  ;[0.05098 0.05098 0.05098] Destroy Text
  (EventDispatchers|AssignDestroyWall (Variables|Default|GetSection) (delegate Custom|DestroyWall_Event)))

(event Custom|DestroyWall_Event
  ;[0.05098 0.05098 0.05098] Destroy Text
  (Actor|DestroyActor))

(event EventBeginPlay
  ;[0.05098 0.05098 0.05098] Update Text
  (Rendering|Components|TextRender|SetText (Variables|Default|GetTextRender) (Utilities|Text|ToText(Integer) (Variables|/Game/Maps/MapObjects/BP_SectionSeparator.BP_SectionSeparator_C|GetNumSpawnPoints (Variables|Default|GetSection))))
  (EventDispatchers|AssignNumSpawnUpdate (Variables|Default|GetSection) (delegate Custom|NumSpawnUpdate_Event))
  ;[0.05098 0.05098 0.05098] Destroy Text
  (EventDispatchers|AssignDestroyWall (Variables|Default|GetSection) (delegate Custom|DestroyWall_Event)))

(fn ConstructionScript)
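; BP_Checkpoint is a map trigger that saves the first-person character's respawn state and can trigger enemy spawning.
; The first character overlap of its Box activates it, caches player references and sets RespawnLocation from RespawnPoint.
; It stores camera relative transform and gravity direction on the player for gravity-aware respawns, refreshing them on later overlaps.
; If SpawnEnemies is set, it calls the SpawnEnemies event and clears the flag.
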(event OnComponentBeginOverlap(Box)
  (params (OverlappedComponent :type Primitive%20Component%20Object%20Reference) (OtherActor :type Actor%20Object%20Reference) (OtherComp :type Primitive%20Component%20Object%20Reference) (OtherBodyIndex :type Integer) (bFromSweep :type Boolean) (SweepResult :type Hit%20Result%20Structure%20%28by%20ref%29))
  (Utilities|FlowControl|Sequence
    (:then_0
      ;[0.05098 0.05098 0.05098] Set Internal Variables
      (if (not (Variables|Default|GetActivated))
        (bind _asbp_first_person_character (Utilities|Casting|CastToBP_FirstPersonCharacter OtherActor))
        (Variables|Default|SetActivated true)
        (Variables|Default|SetPlayer _asbp_first_person_character)
        (Variables|Default|SetFirst%20Person%20Camera (Variables|/Game/FirstPerson/Blueprints/BP_FirstPersonCharacter.BP_FirstPersonCharacter_C|GetFirstPersonCamera _asbp_first_person_character))
        (Variables|Default|SetCharacter%20Movement (Variables|/Script/Engine.Character|GetCharacterMovement _asbp_first_person_character))
        (Variables|/Game/FirstPerson/Blueprints/BP_FirstPersonCharacter.BP_FirstPersonCharacter_C|SetRespawnLocation _asbp_first_person_character (Transformation|GetWorldLocation (Variables|/Script/Engine.Actor|GetRootComponent (Variables|Default|GetRespawnPoint))))))
    (:then_1
      ;[0.05098 0.05098 0.05098] Set Gravitational Variables for Respawn
      (Variables|/Game/FirstPerson/Blueprints/BP_FirstPersonCharacter.BP_FirstPersonCharacter_C|SetCheckpointRelativeLocation (Variables|Default|GetPlayer) (Variables|/Script/Engine.SceneComponent|GetRelativeLocation (Variables|Default|GetFirst%20Person%20Camera)))
      (Variables|/Game/FirstPerson/Blueprints/BP_FirstPersonCharacter.BP_FirstPersonCharacter_C|SetCheckpointRelativeRotation (Variables|Default|GetPlayer) (Variables|/Script/Engine.SceneComponent|GetRelativeRotation (Variables|Default|GetFirst%20Person%20Camera)))
      (Variables|/Game/FirstPerson/Blueprints/BP_FirstPersonCharacter.BP_FirstPersonCharacter_C|SetCheckpointGravityDirection (Variables|Default|GetPlayer) (Class|CharacterMovementComponent|GetGravityDirection (Variables|Default|GetCharacter%20Movement))))
    (:then_2
      ;[0.05098 0.05098 0.05098] Spawn Enemies on Threshold Cross
      (if (Variables|Default|GetSpawnEnemies)
        (Default|CallSpawnEnemiesEvent)
        (Variables|Default|SetSpawnEnemies false)))))

(fn ConstructionScript)
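; BP_SectionSeparator gates a map section, tracking how many enemies from its SpawnPoints remain.
; It starts the count at the spawn point count, decrements it on EnemyDeath and broadcasts each change through the NumSpawnUpdate dispatcher.
; At zero it broadcasts DestroyWall and destroys itself.
; It binds to the first BP_FirstPersonCharacter's PlayerDeath dispatcher to restore the initial count when the player dies.
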(event Custom|PlayerDeath_Event
  ;[0.05098 0.05098 0.05098] Reset Spawned Enemy Count on Player Death
  (Variables|Default|SetNumSpawnPoints (Variables|Default|GetInitialSpawnPoints))
  (Default|CallNumSpawnUpdate))

(event Custom|EnemyDeath
  ;[0.05098 0.05098 0.05098] Update Spawned Enemy Count
  (bind _result (Math|Integer|DecrementInt (Variables|Default|GetNumSpawnPoints))
    (:%20%20
      (Default|CallNumSpawnUpdate)
      (if (== _result 0)
        (Default|CallDestroyWall)
        (Actor|DestroyActor)))))

(event EventBeginPlay
  (bind _spawnpoints (Variables|Default|GetSpawnPoints))
  (bind _returnvalue (Utilities|Array|Length _spawnpoints))
  ;[0.05098 0.05098 0.05098] Initialize Spawned Enemy Count
  (Variables|Default|SetNumSpawnPoints _returnvalue)
  (Variables|Default|SetInitialSpawnPoints _returnvalue)
  (bind _outactors (Actor|GetAllActorsOfClass "/Game/FirstPerson/Blueprints/BP_FirstPersonCharacter.BP_FirstPersonCharacter_C"))
  (EventDispatchers|AssignPlayerDeath (Utilities|Array|Get(acopy) _outactors) (delegate Custom|PlayerDeath_Event))
  (Default|CallNumSpawnUpdate))

(fn ConstructionScript)
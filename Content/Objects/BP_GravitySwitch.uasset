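; BP_GravitySwitch is a single-use switch that, on UseAbility, sets the player's gravity and forward directions and destroys its two cube components.
; Camera roll and height targets come from maps keyed by gravity direction, while view yaw/pitch limits follow the gravity axis, with forward direction also deciding roll sign for sideways gravity.
; SmallestRotation adjusts ±180 angles for the shorter turn, then the ReverseCamera timeline lerps the camera to its targets.
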(event EventUseAbility
  (bind _returnvalue (Game|GetPlayerCameraManager 0))
  (bind _returnvalue_2 (Game|GetPlayerCameraManager 0))
  (bind _returnvalue_3 (Game|GetPlayerCameraManager 0))
  (bind _returnvalue_4 (Game|GetPlayerCameraManager 0))
  (bind _returnvalue_5 (Game|GetPlayerCameraManager 0))
  (bind _returnvalue_6 (Game|GetPlayerCameraManager 0))
  (bind _gravitydirection (Variables|Default|GetGravityDirection))
  (Utilities|FlowControl|Sequence
    (:then_0
      ;[0.05098 0.05098 0.05098] Get reference to player and its components, and variables
      (bind _outactors (Actor|GetAllActorsOfClass "/Game/FirstPerson/Blueprints/BP_FirstPersonCharacter.BP_FirstPersonCharacter_C"))
      (bind _output_get (Variables|Default|SetPlayer (Utilities|Array|Get(acopy) _outactors)))
      (Variables|Default|SetFirst%20Person%20Camera (Actor|GetComponentbyClass _output_get "/Script/Engine.CameraComponent"))
      (Variables|Default|SetCanRotate false)
      (Variables|/Game/FirstPerson/Blueprints/BP_FirstPersonCharacter.BP_FirstPersonCharacter_C|SetForwardDirection (Variables|Default|GetPlayer) (Variables|Default|GetForwardDirection)))
    (:then_1
      ;[0.05098 0.05098 0.05098] Flip gravity of player
      (Class|CharacterMovementComponent|SetGravityDirection (Variables|/Script/Engine.Character|GetCharacterMovement (Variables|Default|GetPlayer)) _gravitydirection)
      (Variables|Default|SetCameraRotation (.Value (Utilities|Map|Find (Variables|Default|GetCameraRotations) _gravitydirection)))
      (Variables|Default|SetCameraLocation (.Value (Utilities|Map|Find (Variables|Default|GetCameraLocations) _gravitydirection))))
    (:then_2
      (Variables|Default|SetCanRotate true)
      (Components|DestroyComponent (Variables|Default|GetCube2))
      (Components|DestroyComponent (Variables|Default|GetCube)))
    (:then_3
      (Utilities|FlowControl|Sequence
        (:then_0
          (if (Utilities|Operators|EqualEqual (Variables|Default|GetGravityDirection) "0.000000,0.000000,1.000000" 0.0)
            (Variables|/Script/Engine.PlayerCameraManager|SetViewYawMax _returnvalue_3 359.9)
            (Variables|/Script/Engine.PlayerCameraManager|SetViewPitchMax _returnvalue_3 89.9)
            (Variables|/Script/Engine.PlayerCameraManager|SetViewYawMin _returnvalue_3 0.0)
            (Variables|/Script/Engine.PlayerCameraManager|SetViewPitchMin _returnvalue_3 -89.9)))
        (:then_1
          (if (Utilities|Operators|EqualEqual (Variables|Default|GetGravityDirection) "0.000000,0.000000,-1.000000" 0.0)
            (Variables|/Script/Engine.PlayerCameraManager|SetViewYawMax _returnvalue_6 359.9)
            (Variables|/Script/Engine.PlayerCameraManager|SetViewPitchMax _returnvalue_6 89.9)
            (Variables|/Script/Engine.PlayerCameraManager|SetViewYawMin _returnvalue_6 0.0)
            (Variables|/Script/Engine.PlayerCameraManager|SetViewPitchMin _returnvalue_6 -89.9)))
        (:then_2
          (if (Utilities|Operators|EqualEqual (Variables|Default|GetGravityDirection) "0.000000,1.000000,0.000000" 0.0)
            (if (Utilities|Operators|EqualEqual (Variables|Default|GetForwardDirection) "1.000000,0.000000,0.000000" 0.0)
              (Variables|/Script/Engine.PlayerCameraManager|SetViewYawMax _returnvalue 89.8 :!label _label)
              (Variables|/Script/Engine.PlayerCameraManager|SetViewPitchMax _returnvalue 359.9)
              (Variables|/Script/Engine.PlayerCameraManager|SetViewYawMin _returnvalue -89.9)
              (Variables|/Script/Engine.PlayerCameraManager|SetViewPitchMin _returnvalue 0.0)
              (else
                (Variables|/Script/Engine.PlayerCameraManager|SetViewYawMax _returnvalue_2 269.9 :!label _label_2)
                (Variables|/Script/Engine.PlayerCameraManager|SetViewPitchMax _returnvalue_2 359.9)
                (Variables|/Script/Engine.PlayerCameraManager|SetViewYawMin _returnvalue_2 89.9)
                (Variables|/Script/Engine.PlayerCameraManager|SetViewPitchMin _returnvalue_2 0.0)
                (Variables|Default|SetCameraRotation (* (Variables|Default|GetCameraRotation) -1.0))))))
        (:then_3
          (if (Utilities|Operators|EqualEqual (Variables|Default|GetGravityDirection) "0.000000,-1.000000,0.000000" 0.0)
            (if (Utilities|Operators|EqualEqual (Variables|Default|GetForwardDirection) "1.000000,0.000000,0.000000" 0.0)
              (goto _label)
              (else
                (goto _label_2)))))
        (:then_4
          (if (Utilities|Operators|EqualEqual (Variables|Default|GetGravityDirection) "1.000000,0.000000,0.000000" 0.0)
            (if (Utilities|Operators|EqualEqual (Variables|Default|GetForwardDirection) "0.000000,1.000000,0.000000" 0.0)
              (Variables|/Script/Engine.PlayerCameraManager|SetViewYawMax _returnvalue_4 179.9 :!label _label_3)
              (Variables|/Script/Engine.PlayerCameraManager|SetViewPitchMax _returnvalue_4 359.9)
              (Variables|/Script/Engine.PlayerCameraManager|SetViewYawMin _returnvalue_4 0.0)
              (Variables|/Script/Engine.PlayerCameraManager|SetViewPitchMin _returnvalue_4 0.0)
              (else
                (Variables|/Script/Engine.PlayerCameraManager|SetViewYawMax _returnvalue_5 359.9 :!label _label_4)
                (Variables|/Script/Engine.PlayerCameraManager|SetViewPitchMax _returnvalue_5 359.9)
                (Variables|/Script/Engine.PlayerCameraManager|SetViewYawMin _returnvalue_5 179.9)
                (Variables|/Script/Engine.PlayerCameraManager|SetViewPitchMin _returnvalue_5 0.0)
                (Variables|Default|SetCameraRotation (* (Variables|Default|GetCameraRotation) -1.0))))))
        (:then_5
          (if (Utilities|Operators|EqualEqual (Variables|Default|GetGravityDirection) "-1.000000,0.000000,0.000000" 0.0)
            (if (Utilities|Operators|EqualEqual (Variables|Default|GetForwardDirection) "0.000000,1.000000,0.000000" 0.0)
              (goto _label_3)
              (else
                (goto _label_4)))))))
    (:then_4
      (Variables|Default|SetCurrentCameraRotation (.roll (Variables|/Script/Engine.SceneComponent|GetRelativeRotation (Variables|Default|GetFirst%20Person%20Camera))))
      (Variables|Default|SetCurrentCameraHeight (.z (Variables|/Script/Engine.SceneComponent|GetRelativeLocation (Variables|Default|GetFirst%20Person%20Camera))))
      (CallFunction|SmallestRotation)
      (bind _camerarotation (Timeline|ReverseCamera Play)
        (:Update
          (Transformation|SetRelativeRotation (Variables|Default|GetFirst%20Person%20Camera) (Math|Rotator|MakeRotator (Math|Float|Lerp (Variables|Default|GetCurrentCameraRotation) (Variables|Default|GetCameraRotation) _camerarotation) 0.0 0.0) false false)
          (Transformation|SetRelativeLocation (Variables|Default|GetFirst%20Person%20Camera) (Math|Vector|MakeVector 0.0 0.0 (Math|Float|Lerp (Variables|Default|GetCurrentCameraHeight) (Variables|Default|GetCameraLocation) _camerarotation)) false false))))))

(fn ConstructionScript
  (|CallParentFunction))

(fn SmallestRotation
  ;[0.05098 0.05098 0.05098] Find the smallest angle of rotation between the current and the future rotation of the camera
  (if (> (Math|Float|Absolute(Float) (- (Variables|Default|GetCameraRotation) (Variables|Default|GetCurrentCameraRotation))) 1.8e+02)
    (Utilities|FlowControl|Sequence
      (:then_0
        (if (== (Math|Float|Absolute(Float) (Variables|Default|GetCameraRotation)) 1.8e+02)
          (Math|Float|NegateFloat (Variables|Default|GetCameraRotation))))
      (:then_1
        (if (== (Math|Float|Absolute(Float) (Variables|Default|GetCurrentCameraRotation)) 1.8e+02)
          (Math|Float|NegateFloat (Variables|Default|GetCurrentCameraRotation)))))))